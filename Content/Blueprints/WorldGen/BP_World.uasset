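; BP_World is a world manager that limits the player's chassis to a circular play area and can trigger island spawning.
; Tick finds the W_CountDown widget, then shows time spent beyond the radius from its own location as text and edge opacity.
; When that time exceeds the limit, it resets the chassis to the origin.
; MakeIsland_Event triggers a random BP_IslandSpawnPoint; its repeat loop is disconnected.
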(event `MakeIsland_Event`
  (bind _outactors (`GameplayStatics.GetAllActorsOfClass` "/Game/Blueprints/WorldGen/BP_IslandSpawnPoint.BP_IslandSpawnPoint_C"))
  (bind _outitem (`KismetArrayLibrary.Array_Random` _outactors))
  (`/Game/Blueprints/WorldGen/BP_IslandSpawnPoint.SpawnIsland_Event` _outitem)
  (`KismetArrayLibrary.Array_RemoveItem` _outactors _outitem))

(event `self.ReceiveBeginPlay`
  (bind _returnvalue (`GameplayStatics.GetActorOfClass` "/Game/Blueprints/Flight/BP_Chassis.BP_Chassis_C"))
  (bind _output_get (set `self.Player` _returnvalue)))

(event `self.ReceiveTick`
  (params (DeltaSeconds :type "Float (single-precision)"))
  (bind _outofboundstime (`self.OutOfBoundsTime`))
  (bind _countdownwidget (`self.CountDownWidget`))
  (if (`KismetSystemLibrary.IsValid` (`self.CountDownWidget`))
    (if (> (`KismetMathLibrary.Distance2D` (`KismetMathLibrary.Conv_VectorToVector2D` (`self.K2_GetActorLocation` (`self.Player`))) (`KismetMathLibrary.Conv_VectorToVector2D` (`self.K2_GetActorLocation`))) (`self.PlayAreaRadius`))
      (set `self.OutOfBoundsTime` (+ _outofboundstime DeltaSeconds))
      (set `/Game/Blueprints/UI/W_CountDown.CountDownText` (`KismetStringLibrary.Conv_DoubleToString` _outofboundstime) _countdownwidget)
      (set `/Game/Blueprints/UI/W_CountDown.EdgeOpacity` (/ _outofboundstime (`self.MaxTimeOutOfBounds`)) _countdownwidget)
      (`KismetSystemLibrary.PrintString` "OUt of bounds")
      (if (> _outofboundstime (`self.MaxTimeOutOfBounds`))
        (bind _returnvalue (`GameplayStatics.GetActorOfClass` "/Game/Blueprints/Flight/BP_Chassis.BP_Chassis_C"))
        (`/Game/Blueprints/Flight/BP_Chassis.Reset Player to Loc` _returnvalue (0.0 0.0 0.0) (0.0 0.0 0.0)))
      (else
        (set `self.OutOfBoundsTime` 0.0)))
    (else
      (bind _foundwidgets (`WidgetBlueprintLibrary.GetAllWidgetsOfClass` "/Game/Blueprints/UI/W_CountDown.W_CountDown_C"))
      (if (> (`KismetArrayLibrary.Array_Length` _foundwidgets) 0)
        (set `self.CountDownWidget` (`|GetArrayItem` _foundwidgets))))))

(fn `UserConstructionScript`)