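; BP_HomeIsland is a world-generation actor for the home island, which changes its look according to its altitude.
; Its construction script reads CloudHeight from the first BP_World actor found in the level and compares it with the actor's Z position.
; At or above that height, the Island component uses the SM_Island mesh; below it, the Berg1 mesh.
; Each mesh gets its own fixed relative scale and rotation.
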(fn `UserConstructionScript`
  (bind _outactors (`GameplayStatics.GetAllActorsOfClass` "/Game/Blueprints/WorldGen/BP_World.BP_World_C"))
  (if (>= (.z (.location (`self.GetTransform`))) (`/Game/Blueprints/WorldGen/BP_World.CloudHeight` (`|GetArrayItem` _outactors)))
    (`StaticMeshComponent.SetStaticMesh` (`self.Island`) "/Game/Art/Meshes/Environment/SM_Island.SM_Island")
    (`SceneComponent.SetRelativeScale3D` (`self.Island`) (10.0 10.0 10.0))
    (`SceneComponent.K2_SetRelativeRotation` (`self.Island`) (struct :`Roll` 90.0) false false)
    (else
      (`StaticMeshComponent.SetStaticMesh` (`self.Island`) "/Game/Art/Meshes/Environment/Berg1.Berg1")
      (`SceneComponent.SetRelativeScale3D` (`self.Island`) (81.0 81.0 81.0))
      (`SceneComponent.K2_SetRelativeRotation` :`self` (`self.Island`)))))