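; BP_WorldOLD builds a spherical world of BP_Island actors around its center at BeginPlay.
; Two polar islands always spawn, while exploratory islands use the intermediate points of an N-point Fibonacci sphere, randomly thinned according to Density.
; Each island is placed at Radius, oriented with Z along its offset from the world actor, stored in Islands and attached to the world.
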(event `self.ReceiveBeginPlay`
  (bind _fibindicies (`self.FibIndicies`))
  (bind _returnvalue (- (`self.N`) 2))
  ;[1 1 1] Creates islands at points on a fibonacci sphere
  ;;[1 1 1] Create 2 polar islands
  (for _index (range 2)
    (bind _returnvalue_2 (* (`KismetMathLibrary.MakeVector` 0.0 0.0 (`KismetMathLibrary.Conv_IntToDouble` (- (* _index 2) 1))) (`self.Radius`)))
    (bind _returnvalue_3 (`|SpawnActorFromClass` "/Game/Blueprints/Core/World/BP_Island.BP_Island_C" (`KismetMathLibrary.MakeTransform` _returnvalue_2 (`KismetMathLibrary.MakeRotFromZ` (- _returnvalue_2 (`self.K2_GetActorLocation`)))) "AlwaysSpawn" "MultiplyWithRoot" null null))
    (`KismetArrayLibrary.Array_Add` (`self.Islands`) _returnvalue_3)
    (`self.K2_AttachToActor` _returnvalue_3 self "None" "KeepRelative" "KeepRelative" "KeepRelative" false))
  ;;[1 1 1] Generate a subset of all points based on density
  (for _index_2 (range 1 (+ _returnvalue 1))
    (`KismetArrayLibrary.Array_Add` (`self.FibIndicies`) _index_2))
  (for _ (range 1 (+ (* _returnvalue (- 1.0 (`self.Density`))) 1))
    (`KismetArrayLibrary.Array_Remove` _fibindicies (`KismetMathLibrary.RandomIntegerInRange` 0 (`KismetArrayLibrary.Array_LastIndex` _fibindicies))))
  ;;[1 1 1] Create exploratory islands
  (for _array_element (`self.FibIndicies`)
    (bind _returnvalue_4 (- (/ (* _array_element 2.0) (- (`self.N`) 1)) 1))
    (bind _returnvalue_5 (`KismetMathLibrary.Sqrt` (- 1.0 (`KismetMathLibrary.Square` _returnvalue_4))))
    (bind _returnvalue_6 (/ (* _array_element 6.2831) 1.618033))
    (bind _returnvalue_7 (* (`KismetMathLibrary.MakeVector` (* _returnvalue_5 (`KismetMathLibrary.Cos` _returnvalue_6)) (* _returnvalue_5 (`KismetMathLibrary.Sin` _returnvalue_6)) _returnvalue_4) (`self.Radius`)))
    (bind _returnvalue_8 (`|SpawnActorFromClass` "/Game/Blueprints/Core/World/BP_Island.BP_Island_C" (`KismetMathLibrary.MakeTransform` _returnvalue_7 (`KismetMathLibrary.MakeRotFromZ` (- _returnvalue_7 (`self.K2_GetActorLocation`)))) "AlwaysSpawn" "MultiplyWithRoot" null null))
    (`KismetArrayLibrary.Array_Add` (`self.Islands`) _returnvalue_8)
    (`self.K2_AttachToActor` _returnvalue_8 self "None" "KeepRelative" "KeepRelative" "KeepRelative" false)))

(fn `UserConstructionScript`)