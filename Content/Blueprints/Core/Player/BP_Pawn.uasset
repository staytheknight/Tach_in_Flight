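; Camera pawn with smoothed zoom, pan and stepped rotation that follows the first BP_Vehicle in the level.
; Inputs set desired zoom (clamped), location and rotation, seeded on BeginPlay and interpolated toward on Tick.
; Tick also looks up the vehicle every frame, overwriting desired location with its mesh position and aligning the spring arm to its pitch and yaw.
; A separate FollowCam function is defined but not called here.
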(event `self.ReceiveBeginPlay`
  ;[1 1 1] Grabs actor location on start play and sets the location desired to prevent the camera from interpolating to desired location on game start
  (set `self.Location_Desired` (`self.K2_GetActorLocation`))
  ;[1 1 1] Grabs Target arm length for spring arm and sets the zoom desired to prevent interpolation to desired zoom on first frame
  (set `self.Zoom_Desired` (`SpringArmComponent.TargetArmLength` (`self.SpringArm`)))
  ;[1 1 1] Sets Rotation desired based on actor rotation on spawn (prevents first frame interpolation)
  (set `self.Rotation_Desired` (`self.K2_GetActorRotation`)))

(event `self.ReceiveTick`
  (params (DeltaSeconds :type "Float (single-precision)"))
  (bind _springarm (`self.SpringArm`))
  (bind _springarm_2 (`self.SpringArm`))
  (bind _returnvalue_roll (`KismetMathLibrary.BreakRotator` (`SceneComponent.K2_GetComponentRotation` _springarm_2)))
  ;[0.394 0.7539 1] Camera Zoom
  ;;[1 1 1] Interpolates Zoom (Smooth zoom instead of incremental)
  (set `SpringArmComponent.TargetArmLength` (`KismetMathLibrary.FInterpTo` (`SpringArmComponent.TargetArmLength` _springarm) (`self.Zoom_Desired`) DeltaSeconds (`self.ZInterpSpeed`)) _springarm)
  ;[1 0.6354 0.6354] Camera Movement Interpolation
  (`self.K2_SetActorLocation` (`KismetMathLibrary.VInterpTo` (`self.K2_GetActorLocation`) (`self.Location_Desired`) DeltaSeconds (`self.MInterpSpeed`)))
  ;[0.4436 1 0.5193] Rotation Interpolation
  (`self.K2_SetActorRotation` (`KismetMathLibrary.RInterpTo` (`self.K2_GetActorRotation`) (`self.Rotation_Desired`) DeltaSeconds (`self.RInterpSpeed`)))
  ;[1 1 1] Bespoke Follow Cam
  (bind _outactors (`GameplayStatics.GetAllActorsOfClass` "/Game/Blueprints/Flight/Unfinished/BP_Vehicle.BP_Vehicle_C"))
  (bind _staticmesh (`/Game/Blueprints/Flight/Unfinished/BP_Vehicle.StaticMesh` (`|GetArrayItem` _outactors)))
  (set `self.Location_Desired` (`SceneComponent.K2_GetComponentLocation` _staticmesh))
  (bind (_returnvalue_roll_2 _returnvalue_pitch _returnvalue_yaw) (`KismetMathLibrary.BreakRotator` (`SceneComponent.K2_GetComponentRotation` _staticmesh)))
  (`SceneComponent.K2_SetRelativeRotation` _springarm_2 (`KismetMathLibrary.MakeRotator` (`KismetMathLibrary.FInterpTo` _returnvalue_roll _returnvalue_roll_2 0.0 5.0) (- _returnvalue_pitch 10.0) _returnvalue_yaw) false false))

(event `InputAxis|InputAxis_Zoom`
  (params (AxisValue :type "Float (single-precision)"))
  ;[0.394 0.7539 1] Camera Zoom
  (set `self.Zoom_Desired` (`KismetMathLibrary.FClamp` (+ (* AxisValue (`self.ZoomScale`)) (`self.Zoom_Desired`)) (`self.ZClampMin`) (`self.ZClampMax`))))

(event `InputAxis|InputAxis_Forward`
  (params (AxisValue :type "Float (single-precision)"))
  ;[1 0.5614 0.5913] Camera Movements (Based on actor vectors not world space - it's what the 'get actor vector' function calls are for)
  (set `self.Location_Desired` (+ (`self.Location_Desired`) (* (* AxisValue (`self.MovementScale`)) (`self.GetActorForwardVector`)))))

(event `InputAxis|InputAxis_Right`
  (params (AxisValue :type "Float (single-precision)"))
  ;[1 0.5614 0.5913] Camera Movements (Based on actor vectors not world space - it's what the 'get actor vector' function calls are for)
  (set `self.Location_Desired` (+ (`self.Location_Desired`) (* (* AxisValue (`self.MovementScale`)) (`self.GetActorRightVector`)))))

(event `InputAction|InputAction_RotationLeft`
  (params (Key :type "Key Structure"))
  ;[0.5624 1 0.6224] Camera Rotation
  (:`Pressed`
    (set `self.Rotation_Desired` (`KismetMathLibrary.ComposeRotators` (`self.Rotation_Desired`) (`KismetMathLibrary.MakeRotator` 0.0 0.0 (- 0.0 (`self.RotationAngle`)))))))

(event `InputAction|InputAction_RotationRight`
  (params (Key :type "Key Structure"))
  ;[0.5624 1 0.6224] Camera Rotation
  (:`Pressed`
    (set `self.Rotation_Desired` (`KismetMathLibrary.ComposeRotators` (`self.Rotation_Desired`) (`KismetMathLibrary.MakeRotator` 0.0 0.0 (`self.RotationAngle`))))))

(fn `FollowCam`
  (params (FollowActor :type "Actor Object Reference"))
  (`self.K2_SetActorLocation` self (`KismetMathLibrary.VInterpTo` (`self.K2_GetActorLocation` self) (`self.K2_GetActorLocation` FollowActor) 0.0 5.0) false false))

(fn `UserConstructionScript`)