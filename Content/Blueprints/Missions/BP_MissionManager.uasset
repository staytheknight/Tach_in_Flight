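; Mission manager for a fish delivery game in which the player flies between islands, collects fish and delivers them to NPCs.
; On BeginPlay it shuffles NPC types across spawns, randomizes item fish, picks a typed NPC, spawns its delivery zone and draws a shuffled fish order.
; Tick trades matching cargo while the player is landed in the zone, blanking filled slots.
; An order with no fish left rerolls item spawns and the mission.
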(event `self.ReceiveBeginPlay`
  (`self.GetPlayer`)
  (`self.GetIslands`)
  (`self.GetNPCsSpawns` false)
  (`self.GetItemSpawns`)
  (`self.PopulateNPCs`)
  (`self.RandomizeFish`)
  (`self.PopulateItemSpawns`)
  (`self.GenerateMission`))

(event `self.ReceiveTick`
  (params (DeltaSeconds :type "Float (single-precision)"))
  (`self.UpdateMission`))

(fn `GenerateMission`
  (locals (MissionItemsNeededLoopCount :type Integer :default 0))
  (bind _fishfordelivery (`self.FishForDelivery`))
  (bind _fishtospawn (`self.FishToSpawn`))
  ;[1 1 1] Sets which npc wants the delivery
  (`self.GetNPCsSpawns` true) ; Repopulate the NPC Spawn list but ignore spawn points with NPC type None.\nThis is to prevent the mission NPC from being a None NPC
  (set `self.MissionNPC` (`KismetArrayLibrary.Array_Random` (`self.NPCsSpawns`)))
  ;[1 1 1] Destroy All exisiting delivery zones before spawning a new one
  (bind _outactors (`GameplayStatics.GetAllActorsOfClass` "/Game/Blueprints/Missions/BP_DeliveryZone.BP_DeliveryZone_C"))
  (for _array_element _outactors
    (`self.K2_DestroyActor` _array_element))
  ;[1 1 1] Spawns Delivery Zone on that NPC
  (bind _returnvalue (`|SpawnActorFromClass` "/Game/Blueprints/Missions/BP_DeliveryZone.BP_DeliveryZone_C" (`KismetMathLibrary.MakeTransform` (`self.K2_GetActorLocation` (`self.MissionNPC`))) "Undefined" "MultiplyWithRoot" null null))
  (set `self.DeliveryZone` _returnvalue)
  ;[0.1094 0.1094 0.1094] Determines which and how many fish needed for delivery - only fish that exist on the map
  (bind _output_get (set `local.MissionItemsNeededLoopCount` (`KismetMathLibrary.RandomIntegerInRange` 1 4))) ; This is here because the following loop \nwill call rand on each loop - this is to\n set a static number
  (`KismetArrayLibrary.Array_Clear` (`self.FishForDelivery`))
  ;;[1 1 1] Adds the fish needed for delivery into an array, shuffles the original array first as trying to get a random element will duplicate the random on each loop sometimes. Shuffling and getting only x works better
  (`KismetArrayLibrary.Array_Shuffle` _fishtospawn)
  (for _index (range (+ _output_get 1))
    (`KismetArrayLibrary.Array_Add` _fishfordelivery (`|GetArrayItem` _fishtospawn _index)))
  (`KismetArrayLibrary.SortByteArray` _fishfordelivery) ; Sorting for display purpouses
)

(fn `GetIslands`
  (bind _outactors (`GameplayStatics.GetAllActorsOfClass` "/Game/Blueprints/WorldGen/BP_Island.BP_Island_C"))
  (set `self.Islands` _outactors))

(fn `GetItemSpawns`
  (bind _outactors (`GameplayStatics.GetAllActorsOfClass` "/Game/Blueprints/Missions/BP_Item.BP_Item_C"))
  (set `self.ItemSpawns` _outactors))

(fn `GetNPCsSpawns`
  (params (IgnoreNPCTypeNone :type Boolean))
  (bind _outactors (`GameplayStatics.GetAllActorsOfClass` "/Game/Blueprints/Missions/BP_NPC.BP_NPC_C"))
  (bind _output_get (set `self.NPCsSpawns` _outactors))
  (if IgnoreNPCTypeNone
    ;[1 1 1] Connect this if you don't want to pick up NPC spawns with no npc type
    (for _array_element _output_get
      (`/Engine/EditorBlueprintResources/StandardMacros.IsValid` _array_element
        (:`Is Valid`
          (if (`|EnumEquality` (`/Game/Blueprints/Missions/BP_NPC.NPCType` _array_element) "NewEnumerator4")
            (`KismetArrayLibrary.Array_RemoveItem` (`self.NPCsSpawns`) _array_element)))))))

(fn `GetPlayer`
  (bind _outactors (`GameplayStatics.GetAllActorsOfClass` "/Game/Blueprints/Flight/BP_Chassis.BP_Chassis_C"))
  (set `self.Player` (`|GetArrayItem` _outactors)))

(fn `PopulateItemSpawns`
  ;[1 1 1] For each item spawn location in the world, set it's fish type to spawn, as well as set hidden in game to visible, and let the sphere collision component accept overlaps (these might have been reset when the player picks them up)
  (for (_array_element _array_index) (`self.ItemSpawns`)
    (set `/Game/Blueprints/Missions/BP_Item.FishType` (`|GetArrayItem` (`self.FishToSpawn`) _array_index) _array_element)
    (`SceneComponent.SetHiddenInGame` (`/Game/Blueprints/Missions/BP_Item.FishBillboardSprite` _array_element) false false)
    (set `PrimitiveComponent.bGenerateOverlapEvents` true (`/Game/Blueprints/Missions/BP_Item.SphereCollision` _array_element))))

(fn `PopulateNPCs`
  (bind _npcsspawns (`self.NPCsSpawns`))
  (`KismetArrayLibrary.Array_Shuffle` _npcsspawns)
  (for (_array_element _array_index) (`self.NPCEnumArray`)
    ;[1 1 1] To Prevent out of bounds array gets
    (if (< _array_index (`KismetArrayLibrary.Array_Length` _npcsspawns))
      (set `/Game/Blueprints/Missions/BP_NPC.NPCType` _array_element (`|GetArrayItem` _npcsspawns _array_index))))
  (for _array_element_2 (`self.Islands`)
    (`/Game/Blueprints/WorldGen/BP_Island.Hide NPCBuildings` _array_element_2)))

(fn `PrintMission`
  (bind _player (`self.Player`))
  (`KismetSystemLibrary.PrintString` (`KismetStringLibrary.Concat_StrStr` "Mission NPC: " (`|GetEnumeratorNameAsString` (`/Game/Blueprints/Missions/BP_NPC.NPCType` (`self.MissionNPC`)))) true false (struct :`G` 0.66 :`B` 1.0 :`A` 1.0) 0.0)
  (for _array_element (`self.FishForDelivery`)
    (`KismetSystemLibrary.PrintString` (`KismetStringLibrary.Concat_StrStr` "Fish Needed: " (`|GetEnumeratorNameAsString` _array_element)) true false (struct :`G` 0.66 :`B` 1.0 :`A` 1.0) 0.0))
  (`KismetSystemLibrary.PrintString` (`KismetStringLibrary.Concat_StrStr` "Cargo Capacity: " (`KismetStringLibrary.Conv_IntToString` (`/Game/Blueprints/Flight/BP_Chassis.CargoCapacity` _player)) " ,Cargo Count: " (`KismetStringLibrary.Conv_IntToString` (`/Game/Blueprints/Flight/BP_Chassis.CargoCount` _player))) true false (struct :`G` 0.66 :`B` 1.0 :`A` 1.0) 0.0))

(fn `RandomizeFish`
  (`KismetArrayLibrary.Array_Clear` (`self.FishToSpawn`))
  (for _ (range (`KismetArrayLibrary.Array_Length` (`self.Islands`)))
    (`KismetArrayLibrary.Array_Add` (`self.FishToSpawn`) (`KismetArrayLibrary.Array_Random` (`self.FishEnumArray`)))))

(fn `UpdateMission`
  (bind _player (`self.Player`))
  (bind _fishfordelivery (`self.FishForDelivery`))
  (bind _cargocontents (`/Game/Blueprints/Flight/BP_Chassis.CargoContents` _player))
  (`|ExecutionSequence`
    (:`then_0`
      ;[1 1 1] If the player is in the delivery zone ,and has landed
      (if (and (`/Game/Blueprints/Missions/BP_DeliveryZone.HasOverlap?` (`self.DeliveryZone`)) (not (`/Game/Blueprints/Flight/BP_Chassis.Flying?` (`self.Player`))))
        ;[1 1 1] Check each item in the cargo of player
        (for _array_element (`/Game/Blueprints/Flight/BP_Chassis.CargoContents` (`self.Player`))
          ;[1 0 0.4937] If item in player cargo is in the delivery list, then remove that item from both lists, and increment cargo capacity
          (if (`KismetArrayLibrary.Array_Contains` (`self.FishForDelivery`) _array_element)
            (`KismetArrayLibrary.Array_Set` _fishfordelivery (`KismetArrayLibrary.Array_Find` _fishfordelivery _array_element) "NewEnumerator4")
            (`KismetArrayLibrary.Array_Remove` _cargocontents (`KismetArrayLibrary.Array_Find` _cargocontents _array_element))
            (`/Engine/EditorBlueprintResources/StandardMacros.DecrementInt` (`/Game/Blueprints/Flight/BP_Chassis.CargoCount` _player))))))
    (:`then_1`
      (`KismetArrayLibrary.Array_Clear` (`self.FishTypeExists`))
      ;[0 0 0] Goes through the fish for delivery array, and checks if each element is a fish type (that is to say not NONE) - the boolean is then stored in a boolean array
      (for (_array_element_2 _array_index) (`self.FishEnumArray`)
        (`KismetArrayLibrary.Array_Set` (`self.FishTypeExists`) _array_index (`KismetArrayLibrary.Array_Contains` (`self.FishForDelivery`) _array_element_2) true))
      ;[1 1 1] If the Delivery list does NOT contain any fish types (the entire array is NONE) - Generate a new mission
      (if (not (`KismetArrayLibrary.Array_Contains` (`self.FishTypeExists`) true))
        (`self.RandomizeFish`)
        (`self.PopulateItemSpawns`)
        (`self.GenerateMission`)))))

(fn `UserConstructionScript`)