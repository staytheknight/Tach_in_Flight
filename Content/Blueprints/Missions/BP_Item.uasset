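; BP_Item is a collectible fish pickup for delivery missions, shown as a billboard sprite coloured by its fish type.
; On BeginPlay it caches the player chassis and mission manager, and every Tick it sets the sprite from FishType.
; On sphere overlap, if cargo has room and the mission wants that type, it adds the fish to the player's cargo.
; It then hides and disables overlaps rather than destroying itself, so other scripts keep their references.
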(event `self.ReceiveBeginPlay`
  (bind _outactors (`GameplayStatics.GetAllActorsOfClass` "/Game/Blueprints/Flight/BP_Chassis.BP_Chassis_C"))
  (set `self.Player` (`|GetArrayItem` _outactors))
  (bind _outactors_2 (`GameplayStatics.GetAllActorsOfClass` "/Game/Blueprints/Missions/BP_MissionManager.BP_MissionManager_C"))
  (set `self.MissionManager` (`|GetArrayItem` _outactors_2)))

(event `self.ReceiveTick`
  (params (DeltaSeconds :type "Float (single-precision)"))
  (`self.ChangeBillboard`))

(event `self.SphereCollision.OnComponentBeginOverlap`
  (params (OverlappedComponent :type "PrimitiveComponent Object Reference") (OtherActor :type "Actor Object Reference") (OtherComp :type "PrimitiveComponent Object Reference") (OtherBodyIndex :type Integer) (bFromSweep :type Boolean) (SweepResult :type "HitResult Structure (by ref)"))
  (bind _player (`self.Player`))
  ;[1 1 1] If the player collides with the item, has cargo capacity AND the mission calls for that type of fish
  (if (and (> (`/Game/Blueprints/Flight/BP_Chassis.CargoCapacity` _player) (`/Game/Blueprints/Flight/BP_Chassis.CargoCount` _player)) (`KismetArrayLibrary.Array_Contains` (`/Game/Blueprints/Missions/BP_MissionManager.FishForDelivery` (`self.MissionManager`)) (`self.FishType`)))
    ;[0.08854 0.08854 0.08854] Then add that fish to the player cargo, reduce their cargo capacity - Then hide the item and disable overlap events - we don't want to destroy the object as it still needs to be referenced by other scripts
    (`KismetArrayLibrary.Array_Add` (`/Game/Blueprints/Flight/BP_Chassis.CargoContents` (`self.Player`)) (`self.FishType`))
    (`/Engine/EditorBlueprintResources/StandardMacros.IncrementInt` (`/Game/Blueprints/Flight/BP_Chassis.CargoCount` (`self.Player`))
      (:`  `
        (`SceneComponent.SetHiddenInGame` (`self.FishBillboardSprite`) true false)
        (set `PrimitiveComponent.bGenerateOverlapEvents` false (`self.SphereCollision`))))))

(fn `ChangeBillboard`
  (bind _fishbillboardsprite (`self.FishBillboardSprite`))
  (switch `/Game/Blueprints/Missions/E_FishTypes` (`self.FishType`)
    (:`NewEnumerator0`
      (`BillboardComponent.SetSprite` _fishbillboardsprite "/Game/Art/Sprites/Fish/Fish_Blue_Filled.Fish_Blue_Filled"))
    (:`NewEnumerator1`
      (`BillboardComponent.SetSprite` _fishbillboardsprite "/Game/Art/Sprites/Fish/Fish_Red_Filled.Fish_Red_Filled"))
    (:`NewEnumerator2`
      (`BillboardComponent.SetSprite` _fishbillboardsprite "/Game/Art/Sprites/Fish/Fish_Green_Filled.Fish_Green_Filled"))
    (:`NewEnumerator3`
      (`BillboardComponent.SetSprite` _fishbillboardsprite "/Game/Art/Sprites/Fish/Fish_Yellow_Filled.Fish_Yellow_Filled"))))

(fn `UserConstructionScript`)