(event `self.ReceiveBeginPlay`
  (`KismetSystemLibrary.Delay` 0.2)
  (bind _outactors (`GameplayStatics.GetAllActorsOfClass` "/Game/Blueprints/Flight/BP_Chassis.BP_Chassis_C"))
  (set `self.BP_Chassis` (`|GetArrayItem` _outactors)))

(event `InputAction|InputAction_Left` :consume false
  (params (Key :type "Key Structure"))
  ;[1 1 1] Rotation of chassis camera
  (:`Pressed`
    (if (`self.BuildMode?`)
      (`SceneComponent.K2_AddRelativeRotation` (`/Game/Blueprints/Flight/BP_Chassis.SpringArm` (`self.BP_Chassis`)) (`KismetMathLibrary.MakeRotator` 0.0 0.0 45.0) false false))))

(event `InputAction|InputAction_Right` :consume false
  (params (Key :type "Key Structure"))
  ;[1 1 1] Rotation of chassis camera
  (:`Pressed`
    (if (`self.BuildMode?`)
      (`SceneComponent.K2_AddRelativeRotation` (`/Game/Blueprints/Flight/BP_Chassis.SpringArm` (`self.BP_Chassis`)) (`KismetMathLibrary.MakeRotator` 0.0 0.0 -45.0) false false))))

(event `InputAction|InputAction_Up` :consume false
  (params (Key :type "Key Structure"))
  (bind _springarm (`/Game/Blueprints/Flight/BP_Chassis.SpringArm` (`self.BP_Chassis`)))
  (bind (_returnvalue_roll _returnvalue_pitch) (`KismetMathLibrary.BreakRotator` (`SceneComponent.K2_GetComponentRotation` _springarm)))
  ;[1 1 1] Rotation of chassis camera
  (:`Pressed`
    (if (`self.BuildMode?`)
      (`SceneComponent.K2_AddLocalRotation` _springarm (`KismetMathLibrary.MakeRotator` 0.0 (`KismetMathLibrary.SelectFloat` 0.0 -45.0 (== _returnvalue_pitch -90.0))) false false))))

(event `InputAction|InputAction_Down` :consume false
  (params (Key :type "Key Structure"))
  (bind _springarm (`/Game/Blueprints/Flight/BP_Chassis.SpringArm` (`self.BP_Chassis`)))
  (bind (_returnvalue_roll _returnvalue_pitch) (`KismetMathLibrary.BreakRotator` (`SceneComponent.K2_GetComponentRotation` _springarm)))
  ;[1 1 1] Rotation of chassis camera
  (:`Pressed`
    (if (`self.BuildMode?`)
      (`SceneComponent.K2_AddLocalRotation` _springarm (`KismetMathLibrary.MakeRotator` 0.0 (`KismetMathLibrary.SelectFloat` 0.0 45.0 (== _returnvalue_pitch 45.0))) false false))))

(event `Key|K`
  (params (Key :type "Key Structure"))
  (:`Pressed`
    (if (`self.BuildMode?`)
      (`self.RemoveAllAttachedParts`))))

(event `Key|J`
  (params (Key :type "Key Structure"))
  (bind _bp_chassis (`self.BP_Chassis`))
  (:`Pressed`
    (if (`self.BuildMode?`)
      (`/Game/Blueprints/Flight/BP_Chassis.CreateDefaultVehicle` _bp_chassis)
      (`/Game/Blueprints/Flight/BP_Chassis.RefreshVehicleParameters` _bp_chassis))))

(fn `DeleteOccupiedConnectorSockets`
  (params (`Scene Components` :type "Array of SceneComponent Object Reference"))
  (locals (Component :type "SceneComponent Object Reference"))
  (bind _returnvalue (`SceneComponent.GetAttachSocketName` (`local.Component`)))
  (for _array_element `Scene Components`
    ;[1 1 1] If the component is NOT a ConnectorSocket Visual
    ; AND it is connected to a socket
    (bind _output_get (set `local.Component` _array_element))
    (`/Engine/EditorBlueprintResources/StandardMacros.IsValid` _output_get
      (:`Is Valid`
        ;[0 0 0] Deletes Connector Socket Visuals for Connector components that are attached to an opposite connector component
        ;;[1 1 1] If the component is owned by BP_Connector
        (if (== (`GameplayStatics.GetObjectClass` (`ActorComponent.GetOwner` (`local.Component`))) "/Game/Blueprints/BuildMode/Parts/BP_Connector.BP_Connector_C")
          ;;[1 1 1] Then get all of it's children
          (for _array_element_2 (`SceneComponent.GetChildrenComponents` (`local.Component`) false)
            ;;[1 1 1] If the Child component is a connector socket visual , AND it has the opposite socket name of the attached parent
            (bind _returnvalue_2 (`|GetDataTableRow` "/Game/Blueprints/BuildMode/DT_ConnectorSocketOppositeNames.DT_ConnectorSocketOppositeNames" (`SceneComponent.GetAttachSocketName` (`local.Component`)))
              (:`then`
                ;;[1 1 1] THEN delete the ConnectorSocket visual
                (if (and (`ActorComponent.ComponentHasTag` _array_element_2 "ConnectorVisual") (== (break `/Game/Blueprints/BuildMode/S_OppositeSocket` _returnvalue_2) (`SceneComponent.GetAttachSocketName` _array_element_2)))
                  (bind _asbp_connector_socket (cast `/Game/Blueprints/BuildMode/BP_ConnectorSocket` (`ActorComponent.GetOwner` _array_element_2)))
                  (`/Game/Blueprints/BuildMode/BP_ConnectorSocket.DestroySelf` _asbp_connector_socket)
                  (if (and (not (`ActorComponent.ComponentHasTag` (`local.Component`) "ConnectorVisual")) (!= _returnvalue "None")) :!label _label
                    ;[1 1 1] Then get the parent that component is attached to and iterate through all the children of that parent (Some of it's children will be connector socket visuals)
                    (for _array_element_3 (`SceneComponent.GetChildrenComponents` (`SceneComponent.GetAttachParent` (`local.Component`)) false)
                      ;[1 1 1] THEN delete the ConnectorSocket visual
                      (if (and (`ActorComponent.ComponentHasTag` _array_element_3 "ConnectorVisual") (== (`SceneComponent.GetAttachSocketName` _array_element_3) _returnvalue))
                        (bind _asbp_connector_socket_2 (cast `/Game/Blueprints/BuildMode/BP_ConnectorSocket` (`ActorComponent.GetOwner` _array_element_3)))
                        (`/Game/Blueprints/BuildMode/BP_ConnectorSocket.DestroySelf` _asbp_connector_socket_2))))))))
          (else
            (goto _label)))))))

(fn `DestroyAllConnectorSockets`
  ;[1 1 1] Goes through the component list and destroys any connectorsocket visuals
  (`self.GetAllComponents` true)
  (for _array_element (`self.Components`)
    (`/Engine/EditorBlueprintResources/StandardMacros.IsValid` _array_element
      (:`Is Valid`
        (if (`ActorComponent.ComponentHasTag` _array_element "ConnectorVisual")
          (bind _asbp_connector_socket (cast `/Game/Blueprints/BuildMode/BP_ConnectorSocket` (`ActorComponent.GetOwner` _array_element)))
          (`/Game/Blueprints/BuildMode/BP_ConnectorSocket.DestroySelf` _asbp_connector_socket))))))

(fn `DisplayConnectors`
  (locals (SocketNames :type "Array of Name") (Component :type "SceneComponent Object Reference"))
  (bind _rootcomponent (`Actor.RootComponent` (`self.BP_Chassis`)))
  (`self.GetAllComponents` true)
  ;[1 1 1] Iterate through all components
  (for _array_element (`self.Components`)
    (bind _output_get (set `local.Component` _array_element))
    ;[1 1 1] If the Component is a BP_Connector
    (if (== (`GameplayStatics.GetObjectClass` (`ActorComponent.GetOwner` _output_get)) "/Game/Blueprints/BuildMode/Parts/BP_Connector.BP_Connector_C")
      ;[1 1 1] Go through all the children of BP_Connector to find the mesh with the sockets
      (for _array_element_2 (`SceneComponent.GetChildrenComponents` (`local.Component`) false)
        (bind _returnvalue (`SceneComponent.GetAllSocketNames` _array_element_2))
        ;[1 1 1] The mesh with sockets is the only child component of BP_Connector with sockets, the socket name list will be greater than 0 - set that as the new socket name array
        (if (> (`KismetArrayLibrary.Array_Length` _returnvalue) 0)
          (set `local.SocketNames` _returnvalue)))
      ;[1 1 1] See if BP_Connector is connected to something else through a socket, and then remove the opposite socket from the list (this is to stop doubling up socket connector visuals)
      (bind _returnvalue_2 (`|GetDataTableRow` "/Game/Blueprints/BuildMode/DT_ConnectorSocketOppositeNames.DT_ConnectorSocketOppositeNames" (`SceneComponent.GetAttachSocketName` (`local.Component`)))
        (:`then`
          (`KismetArrayLibrary.Array_RemoveItem` (`local.SocketNames`) (break `/Game/Blueprints/BuildMode/S_OppositeSocket` _returnvalue_2))
          ;[1 1 1] Then get all children components of BP_Connector (connected pieces), and remove the socket they are connected to from the list
          (for _array_element_3 (`SceneComponent.GetChildrenComponents` (`local.Component`) false)
            (`KismetArrayLibrary.Array_RemoveItem` (`local.SocketNames`) (`SceneComponent.GetAttachSocketName` _array_element_3)))
          ;[1 1 1] Once all children have been iterated through, the list of unocuppied sockets will be iterated through and sockets visuals will be added
          (for _array_element_4 (`local.SocketNames`)
            _)))))
  ;[0.9516 1 0.9439] Adding connector visuals to the root connector
  (for _array_element_5 (`SceneComponent.GetAllSocketNames` _rootcomponent)
    (bind _returnvalue_3 (`|SpawnActorFromClass` "/Game/Blueprints/BuildMode/BP_ConnectorSocket.BP_ConnectorSocket_C" (`KismetMathLibrary.MakeTransform` (0.0 0.0 0.0)) "AlwaysSpawn" "MultiplyWithRoot" null null))
    (`self.K2_AttachToComponent` _returnvalue_3 _rootcomponent _array_element_5 "KeepRelative" "KeepRelative" "KeepWorld" true))
  (`self.GetAllComponents` true)
  (`self.DeleteOccupiedConnectorSockets` (`self.Components`)))

(fn `EnterBuildMode`
  (bind _returnvalue (`GameplayStatics.GetPlayerController` 0))
  (bind _returnvalue_2 (`GameplayStatics.GetPlayerController` 0))
  (bind _bp_chassis (`self.BP_Chassis`))
  (set `self.BuildMode?` true)
  (set `SpringArmComponent.TargetArmLength` 1000.0 (`/Game/Blueprints/Flight/BP_Chassis.SpringArm` (`self.BP_Chassis`))) ; Should set the target length to the size of the vehicle
  (`self.DisableInput` (`self.BP_Chassis`) _returnvalue_2)
  (`self.EnableInput` _returnvalue_2)
  (set `/Game/Blueprints/Flight/BP_Chassis.CurrentSpeed` 0.0 _bp_chassis)
  (set `/Game/Blueprints/Flight/BP_Chassis.CurrentSpeed` 0.0 _bp_chassis)
  (set `PlayerController.bEnableClickEvents` true _returnvalue)
  (set `PlayerController.bEnableMouseOverEvents` true _returnvalue)
  (`self.DisplayConnectors`))

(fn `ExitBuildMode`
  (bind _returnvalue (`GameplayStatics.GetPlayerController` 0))
  (bind _springarm (`/Game/Blueprints/Flight/BP_Chassis.SpringArm` (`self.BP_Chassis`)))
  (set `self.BuildMode?` false)
  (`SceneComponent.K2_SetRelativeRotation` _springarm (`KismetMathLibrary.MakeRotator` 0.0) false false)
  (set `SpringArmComponent.TargetArmLength` 800.0 _springarm) ; Will need to interp for a smoother transition
  (`self.DisableInput` _returnvalue)
  (`self.EnableInput` (`self.BP_Chassis`) _returnvalue)
  (set `PlayerController.bEnableClickEvents` false _returnvalue)
  (set `PlayerController.bEnableMouseOverEvents` false _returnvalue)
  (`self.DestroyAllConnectorSockets`))

(fn `GetAllComponents`
  (params (GetDescendants :type Boolean))
  (bind _rootcomponent (`Actor.RootComponent` (`self.BP_Chassis`)))
  ;[1 1 1] Gets all components of BP_Chassis including root mesh - adds it to an array
  (`KismetArrayLibrary.Array_Clear` (`self.Components`))
  (bind _output_get (set `self.Components` (`SceneComponent.GetChildrenComponents` _rootcomponent GetDescendants)))
  (`KismetArrayLibrary.Array_Add` _output_get _rootcomponent) ; Adding root scene component as it was not captured during children get
)

(fn `RemoveAllAttachedParts`
  (bind _bp_chassis (`self.BP_Chassis`))
  (bind _attachedcomponents (`/Game/Blueprints/Flight/BP_Chassis.AttachedComponents` _bp_chassis))
  (for _array_element _attachedcomponents
    (`/Engine/EditorBlueprintResources/StandardMacros.IsValid` _array_element
      (:`Is Valid`
        (`self.K2_DestroyActor` _array_element))))
  (`KismetArrayLibrary.Array_Clear` _attachedcomponents)
  (`self.DisplayConnectors`)
  (`/Game/Blueprints/Flight/BP_Chassis.RefreshVehicleParameters` _bp_chassis))

(fn `UserConstructionScript`)