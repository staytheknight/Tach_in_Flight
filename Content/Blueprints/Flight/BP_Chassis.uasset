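; Player-controlled plane chassis with arcade flight, stalling and landing.
; Input axes drive thrust, yaw, pitch and roll, rotating the actor and animating rudder, elevators and ailerons.
; Each tick, speed interpolates toward thrust using drag, then a swept move applies gravity that fades with speed, with pitch raising the stall threshold.
; A downward trace levels and lands it at low speed; hits in flight reflect its heading, toggling physics to prevent spins.
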(event `self.ReceiveBeginPlay`
  ;[1 1 1] Sets Min Thurst to Not Fall Original to current Min Thurst to Not Fall for Stall calculations
  (bind _output_get (set `self.MinThrustToNotFallOriginal` (`self.MinThrustToNotFall`)))
  ;[1 0.5236 0.3214] Sets the plane to flying on game start - can remove
  (bind _output_get_2 (set `self.ThrustSpeed` _output_get))
  (set `self.CurrentSpeed` _output_get_2)
  (set `self.LandingZOffset` 300.0) ; How far below the chassis the landing gear is
)

(event `self.ReceiveTick`
  (params (DeltaSeconds :type "Float (single-precision)"))
  (`|ExecutionSequence`
    (:`then_0`
      (`self.UpdatePosition` DeltaSeconds)
      (`self.LandingTrace` "None" (`self.LandingZOffset`))
      (if (`self.Flying?`)
        (set `self.Gravity` (`KismetMathLibrary.FInterpTo` (`self.Gravity`) 981.0 (`GameplayStatics.GetWorldDeltaSeconds`) 1.0))
        (else
          (set `self.Gravity` 0.0))))
    (:`then_1`
      (if (`self.PrintVariables?`)
        (`self.PrintVariables`)))))

(event `InputAxis|InputAxis_Forward_Arrows`
  (params (AxisValue :type "Float (single-precision)"))
  (set `self.ThrustSpeed` (`KismetMathLibrary.FClamp` (+ (* AxisValue (`GameplayStatics.GetWorldDeltaSeconds`) (`self.ThrustMultiplier`)) (`self.ThrustSpeed`)) (`KismetMathLibrary.SelectFloat` 0.0 -1000.0 (`self.Flying?`)) (`self.MaxThrustSpeed`))))

(event `InputAxis|InputAxis_Right`
  (params (AxisValue :type "Float (single-precision)"))
  (`self.UpdateYaw` (`GameplayStatics.GetWorldDeltaSeconds`) AxisValue))

(event `InputAxis|InputAxis_Forward`
  (params (AxisValue :type "Float (single-precision)"))
  (`self.UpdatePitch` (`GameplayStatics.GetWorldDeltaSeconds`) (select `bool` (`self.InvertPitch?`) :`false` (`KismetMathLibrary.FClamp` AxisValue (`KismetMathLibrary.SelectFloat` -1.0 0.0 (`self.Flying?`))) :`true` (`KismetMathLibrary.FClamp` AxisValue -1.0 (`KismetMathLibrary.SelectFloat` 1.0 0.0 (`self.Flying?`))))))

(event `InputAxis|InputAxis_QE`
  (params (AxisValue :type "Float (single-precision)"))
  (`self.UpdateRoll` (`GameplayStatics.GetWorldDeltaSeconds`) (`KismetMathLibrary.SelectFloat` AxisValue 0.0 (`self.Flying?`))))

(event `self.Chassis.OnComponentHit`
  (params (HitComponent :type "PrimitiveComponent Object Reference") (OtherActor :type "Actor Object Reference") (OtherComp :type "PrimitiveComponent Object Reference") (NormalImpulse :type "Vector Structure") (Hit :type "HitResult Structure (by ref)"))
  ;[1 1 1] Reflects the vehicle on hit
  (if (`self.Flying?`)
    (`self.K2_SetActorRotation` (`KismetMathLibrary.Conv_VectorToRotator` (`KismetMathLibrary.GetReflectionVector` (`SceneComponent.GetForwardVector` (`self.Chassis`)) Hit_Normal)))
    ;;[1 0.04544 0] This is a bit of a hack, it's to prevent the vehicle from going into really intense unrecoverable spins when colliding at high speeds
    (`PrimitiveComponent.SetSimulatePhysics` (`self.Chassis`) false)
    (`PrimitiveComponent.SetSimulatePhysics` (`self.Chassis`) true)))

(fn `LandingTrace`
  (params (Debug :type "EDrawDebugTrace Enum" :default "None") (Offset :type "Float (double-precision)"))
  (bind (_returnvalue_location _returnvalue_rotation _returnvalue_scale) (`KismetMathLibrary.BreakTransform` (`self.GetTransform`)))
  (bind (_returnvalue_roll _returnvalue_pitch _returnvalue_yaw) (`KismetMathLibrary.BreakRotator` (`self.K2_GetActorRotation`)))
  (bind _returnvalue (`SceneComponent.K2_GetComponentLocation` (`self.Chassis`)))
  ;[1 1 1] Line trace from center of chassis to a specified z offset
  (bind (_outhit _returnvalue_2) (`KismetSystemLibrary.LineTraceSingle` _returnvalue (- _returnvalue (`KismetMathLibrary.MakeVector` 0.0 0.0 Offset)) "TraceTypeQuery1" false (`|MakeArray` self :!type "Actor Object Reference") Debug))
  ;[1 0.4658 0.3153] Can only land if speed is low enough
  ;
  ; ISSUES with buggy behaviour if hitting a surface while going too fast
  (if _returnvalue_2
    (if (== (`KismetMathLibrary.MapRangeClamped` (`self.CurrentSpeed`) (`self.TargetSpeedForLanding`) (`self.MaxThrustSpeed`) 0.0 1.0) 0.0)
      ;[1 1 1] Align Vehicle with floor.
      ; Custom variables instead of normals
      ; Rotation is only retained for Yaw
      ; Location includes Z Offset
      (set `self.Flying?` false)
      (`self.K2_SetActorRelativeTransform` (`KismetMathLibrary.MakeTransform` (`KismetMathLibrary.VInterpTo` (`self.K2_GetActorLocation`) (+ (`.TraceEnd` (`GameplayStatics.BreakHitResult` _outhit)) (`KismetMathLibrary.MakeVector` 0.0 0.0 (`self.LandingZOffset`))) (`GameplayStatics.GetWorldDeltaSeconds`) (`self.LandingInterpSpeed`)) (`KismetMathLibrary.MakeRotator` 0.0 0.0 _returnvalue_yaw) _returnvalue_scale))
      (else
        (set `self.Flying?` true :!label _label)))
    (else
      (goto _label))))

(fn `PrintVariables`
  (`|ExecutionSequence`
    (:`then_0`
      (`KismetSystemLibrary.PrintString` (`KismetStringLibrary.Concat_StrStr` "Thrust Speed: " (`KismetStringLibrary.Conv_DoubleToString` (`self.ThrustSpeed`))) true true (struct :`G` 0.66 :`B` 1.0 :`A` 1.0) 0.0))
    (:`then_1`
      (`KismetSystemLibrary.PrintString` (`KismetStringLibrary.Concat_StrStr` "Current Speed: " (`KismetStringLibrary.Conv_DoubleToString` (`self.CurrentSpeed`))) true true (struct :`G` 0.66 :`B` 1.0 :`A` 1.0) 0.0))
    (:`then_2`
      (`KismetSystemLibrary.PrintString` (`KismetStringLibrary.Concat_StrStr` "Applied Gravity: " (`KismetStringLibrary.Conv_DoubleToString` (`self.AppliedGravity`))) true true (struct :`G` 0.66 :`B` 1.0 :`A` 1.0) 0.0))))

(fn `Stall`
  (bind (_returnvalue_roll _returnvalue_pitch) (`KismetMathLibrary.BreakRotator` (`SceneComponent.K2_GetComponentRotation` (`self.Chassis`))))
  (set `self.MinThrustToNotFall` (`KismetMathLibrary.MapRangeClamped` (`KismetMathLibrary.Abs` _returnvalue_pitch) 0.0 90.0 (`self.MinThrustToNotFallOriginal`) (`self.MaxThrustSpeed`))))

(fn `UpdatePitch`
  (params (DeltaSeconds :type "Float (double-precision)") (Pitch :type "Float (double-precision)"))
  (bind _maxelevatorpitch (`self.MaxElevatorPitch`))
  (bind _maxelevatorpitch_2 (`self.MaxElevatorPitch`))
  (if (`self.InvertPitch?`)
    (bind _result (`/Engine/EditorBlueprintResources/StandardMacros.NegateFloat` Pitch)
      (:`  `
        (set `self.TargetPitch` _result)))
    (else
      (set `self.TargetPitch` Pitch)))
  (bind _output_get (set `self.CurrentPitch` (`KismetMathLibrary.FInterpTo` (`self.CurrentPitch`) (`self.TargetPitch`) (`local.DeltaSeconds`) (`self.PitchInterpSpeed`))))
  (`self.K2_AddActorLocalRotation` (`KismetMathLibrary.MakeRotator` 0.0 (* _output_get (`local.DeltaSeconds`) (`self.PitchMultiplier`))))
  ;[1 1 1] Elevator Animations
  (`SceneComponent.K2_SetRelativeRotation` (`self.WingL2`) (`KismetMathLibrary.MakeRotator` 0.0 (`KismetMathLibrary.MapRangeClamped` (`self.CurrentPitch`) -1.0 1.0 _maxelevatorpitch (`self.NegateFloat` _maxelevatorpitch))) false false) ; Roll and pitch are hard coded - there is\nprobably a way to get it dynamically, to \nmatch what the transform of the model is\nbut I can't get it to work without thing\nspinning out of control
  (`SceneComponent.K2_SetRelativeRotation` (`self.WingR1`) (`KismetMathLibrary.MakeRotator` 0.0 (`KismetMathLibrary.MapRangeClamped` (`self.CurrentPitch`) -1.0 1.0 _maxelevatorpitch_2 (`self.NegateFloat` _maxelevatorpitch_2))) false false) ; Roll and pitch are hard coded - there is\nprobably a way to get it dynamically, to \nmatch what the transform of the model is\nbut I can't get it to work without thing\nspinning out of control
)

(fn `UpdatePosition`
  (params (DeltaSeconds :type "Float (double-precision)"))
  (locals (`New Position` :type "Vector Structure"))
  (bind (_new_position_x _new_position_y _new_position_z) (`KismetMathLibrary.BreakVector` (`local.New Position`)))
  (set `self.CurrentSpeed` (`KismetMathLibrary.FInterpTo` (`self.CurrentSpeed`) (`self.ThrustSpeed`) (`local.DeltaSeconds`) (`self.Drag`)))
  ;[1 1 1] Calculates new position based on current speed
  (set `local.New Position` (* (`self.GetActorForwardVector`) (* (`self.CurrentSpeed`) (`local.DeltaSeconds`))))
  ;[1 1 1] Calculate Applied Gravity
  (`self.Stall`)
  (set `self.AppliedGravity` (`KismetMathLibrary.MapRangeClamped` (`self.CurrentSpeed`) 0.0 (`self.MinThrustToNotFall`) (`self.Gravity`)))
  ;[1 1 1] Update Position
  (`self.K2_AddActorWorldOffset` (`KismetMathLibrary.MakeVector` _new_position_x _new_position_y (- _new_position_z (* (`self.AppliedGravity`) (`local.DeltaSeconds`)))) true))

(fn `UpdateRoll`
  (params (DeltaSeconds :type "Float (double-precision)") (Roll :type "Float (double-precision)"))
  (bind _maxaileronpitch (`self.MaxAileronPitch`))
  (bind _maxaileronpitch_2 (`self.MaxAileronPitch`))
  (if (`self.InvertRoll?`)
    (bind _result (`/Engine/EditorBlueprintResources/StandardMacros.NegateFloat` Roll)
      (:`  `
        (set `self.TargetRoll` _result)))
    (else
      (set `self.TargetRoll` Roll)))
  (bind _output_get (set `self.CurrentRoll` (`KismetMathLibrary.FInterpTo` (`self.CurrentRoll`) (`self.TargetRoll`) (`local.DeltaSeconds`) (`self.RollInterpSpeed`))))
  (`self.K2_AddActorLocalRotation` (`KismetMathLibrary.MakeRotator` (* _output_get (`local.DeltaSeconds`) (`self.RollMultiplier`))))
  ;[1 1 1] Aileron Animation
  (`SceneComponent.K2_SetRelativeRotation` (`self.WingL`) (`KismetMathLibrary.MakeRotator` 0.0 (`KismetMathLibrary.MapRangeClamped` (`self.CurrentRoll`) -1.0 1.0 _maxaileronpitch (`self.NegateFloat` _maxaileronpitch))) false false) ; Roll and pitch are hard coded - there is\nprobably a way to get it dynamically, to \nmatch what the transform of the model is\nbut I can't get it to work without thing\nspinning out of control
  (`SceneComponent.K2_SetRelativeRotation` (`self.WingR`) (`KismetMathLibrary.MakeRotator` 0.0 (`KismetMathLibrary.MapRangeClamped` (`self.CurrentRoll`) -1.0 1.0 (`self.NegateFloat` _maxaileronpitch_2) _maxaileronpitch_2)) false false) ; Roll and pitch are hard coded - there is\nprobably a way to get it dynamically, to \nmatch what the transform of the model is\nbut I can't get it to work without thing\nspinning out of control
)

(fn `UpdateYaw`
  (params (DeltaSeconds :type "Float (double-precision)") (Yaw :type "Float (double-precision)"))
  (bind _maxrudderyaw (`self.MaxRudderYaw`))
  (if (`self.InvertYaw?`)
    (bind _result (`/Engine/EditorBlueprintResources/StandardMacros.NegateFloat` Yaw)
      (:`  `
        (set `self.TargetYaw` _result)))
    (else
      (bind _output_get (set `self.TargetYaw` Yaw))))
  (bind _output_get_2 (set `self.CurrentYaw` _output_get))
  (`self.K2_AddActorLocalRotation` (`KismetMathLibrary.MakeRotator` 0.0 0.0 (* _output_get_2 (`local.DeltaSeconds`) (`self.YawMultiplier`))))
  ;[1 1 1] Rudder Animations
  (`SceneComponent.K2_SetRelativeRotation` (`self.Rudder`) (`KismetMathLibrary.MakeRotator` 90.0 90.0 (`KismetMathLibrary.MapRangeClamped` (`self.CurrentYaw`) -1.0 1.0 _maxrudderyaw (`self.NegateFloat` _maxrudderyaw))) false false) ; Roll and pitch are hard coded - there is\nprobably a way to get it dynamically, to \nmatch what the transform of the model is\nbut I can't get it to work without thing\nspinning out of control
)

(fn `UserConstructionScript`)