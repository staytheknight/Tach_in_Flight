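; BP_ConnectorSocket is a flight-part socket actor whose static mesh pulses continuously in size.
; Every Tick calls ThrobMesh, which grows the mesh's world scale by GrowthScale until X exceeds MaxScale, then shrinks it to MinScale and repeats.
; The Growing flag holds the direction, and the step is per frame without delta time, so pulse speed follows frame rate.
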(event `self.ReceiveTick`
  (params (DeltaSeconds :type "Float (single-precision)"))
  (`self.ThrobMesh`))

(fn `ThrobMesh`
  (bind _returnvalue_x (`KismetMathLibrary.BreakVector` (`SceneComponent.K2_GetComponentScale` (`self.StaticMesh`))))
  (if (and (<= (.x (`SceneComponent.K2_GetComponentScale` (`self.StaticMesh`))) (`self.MaxScale`)) (`self.Growing?`))
    (`SceneComponent.SetWorldScale3D` (`self.StaticMesh`) (+ (`SceneComponent.K2_GetComponentScale` (`self.StaticMesh`)) (`self.GrowthScale`)))
    (else
      (set `self.Growing?` false)
      (`SceneComponent.SetWorldScale3D` (`self.StaticMesh`) (- (`SceneComponent.K2_GetComponentScale` (`self.StaticMesh`)) (`self.GrowthScale`)))
      (if (and (<= _returnvalue_x (`self.MinScale`)) (not (`self.Growing?`)))
        (set `self.Growing?` true)))))

(fn `UserConstructionScript`)