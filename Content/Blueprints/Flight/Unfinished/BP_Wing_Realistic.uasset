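; Experimental physics-driven wing actor that approximates flight by applying thrust, drag, lift and gravity forces to its static mesh each tick.
; Axis input adjusts a clamped throttle that drives planar forward force, and an action input adds a forward impulse.
; Planar speed from the change in location feeds lift and drag, both simplified to ½ρv² without area or coefficient terms.
; CalculateForces also prints debug values on screen.
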(event `self.ReceiveBeginPlay`
  (set `self.PrevActorLoc` (`SceneComponent.K2_GetComponentLocation` (`self.StaticMesh`))))

(event `self.ReceiveTick`
  (params (DeltaSeconds :type "Float (single-precision)"))
  (`PrimitiveComponent.AddForce` (`self.StaticMesh`) (`self.CalculateForces` (`self.GravitationForceEstimate`) DeltaSeconds) "None" false)
  (set `self.PrevActorLoc` (`SceneComponent.K2_GetComponentLocation` (`self.StaticMesh`))))

(event `InputAxis|InputAxis_Forward_Arrows`
  (params (AxisValue :type "Float (single-precision)"))
  (`self.ChangeThrottle` AxisValue))

(event `InputAction|InputAction_Impulse`
  (params (Key :type "Key Structure"))
  (bind _impulse_strength (`self.Impulse Strength`))
  (bind (_returnvalue_x _returnvalue_y) (`KismetMathLibrary.BreakVector` (`SceneComponent.GetForwardVector` (`self.StaticMesh`))))
  (:`Pressed`
    (`PrimitiveComponent.AddImpulse` (`self.StaticMesh`) (`KismetMathLibrary.MakeVector` (* _returnvalue_x _impulse_strength) (* _returnvalue_y _impulse_strength)) "None" false)))

(fn `CalculateDrag`
  (params (`Obj Velocity` :type "Float (double-precision)") (DensityOfMedium :type "Float (double-precision)"))
  (returns (`Drag Force` :type "Float (double-precision)"))
  (return (* (`KismetMathLibrary.MultiplyMultiply_FloatFloat` `Obj Velocity` 2.0) (* DensityOfMedium 0.5))))

(fn `CalculateForces`
  (params (GraviationForce :type "Float (double-precision)") (DeltaSeconds :type "Float (double-precision)"))
  (returns (Vector :type "Vector Structure"))
  (locals (ThrottleForce :type "Float (double-precision)" :default 50000.0))
  (bind _velocity (`self.CalculatePlanarVelocity` DeltaSeconds))
  (bind _air_density (`self.AIR_DENSITY`))
  (bind _drag_force (`self.CalculateDrag` _velocity _air_density))
  (bind (_returnvalue_x _returnvalue_y) (`KismetMathLibrary.BreakVector` (`SceneComponent.GetForwardVector` (`self.StaticMesh`))))
  (bind _liftforce (`self.CalculateLiftForce` _velocity _air_density))
  (bind _returnvalue (+ GraviationForce _liftforce))
  (bind _returnvalue_2 (- (* (`self.Throttle`) (`local.ThrottleForce`)) _drag_force))
  (bind _returnvalue_3 (* _returnvalue_2 _returnvalue_x))
  (bind _returnvalue_4 (* _returnvalue_2 _returnvalue_y))
  (`|ExecutionSequence`
    (:`then_0`
      (if true
        (`|ExecutionSequence`
          (:`then_0`
            (if true
              (`KismetSystemLibrary.PrintString` (`KismetStringLibrary.Concat_StrStr` "Velocity: " (`KismetStringLibrary.Conv_DoubleToString` _velocity) " ,Lift Force: " (`KismetStringLibrary.Conv_DoubleToString` _liftforce) " ,Total Z Force: " (`KismetStringLibrary.Conv_DoubleToString` _returnvalue) " ,Drag Force: " (`KismetStringLibrary.Conv_DoubleToString` _drag_force)))))
          (:`then_1`
            (if true
              (`KismetSystemLibrary.PrintString` (`KismetStringLibrary.Concat_StrStr` "Forward Vector, x: " (`KismetStringLibrary.Conv_DoubleToString` _returnvalue_x) " ,y: " (`KismetStringLibrary.Conv_DoubleToString` _returnvalue_y)))))
          (:`then_2`
            (if true
              (`KismetSystemLibrary.PrintString` (`KismetStringLibrary.Concat_StrStr` "Forward Force, x: " (`KismetStringLibrary.Conv_DoubleToString` _returnvalue_3) " ,y: " (`KismetStringLibrary.Conv_DoubleToString` _returnvalue_4)) true true (struct :`R` 1.0 :`G` 0.405428 :`B` 0.435284 :`A` 1.0)))))))
    (:`then_1`
      (return (`KismetMathLibrary.MakeVector` _returnvalue_3 _returnvalue_4 _returnvalue)))))

(fn `CalculateLiftForce`
  (params (ObjVelocity :type "Float (double-precision)") (DensityOfMedium :type "Float (double-precision)"))
  (returns (LiftForce :type "Float (double-precision)"))
  (return (* (`KismetMathLibrary.MultiplyMultiply_FloatFloat` ObjVelocity 2.0) (* DensityOfMedium 0.5))))

(fn `CalculatePlanarVelocity`
  (params (`Delta Seconds` :type "Float (double-precision)"))
  (returns (Velocity :type "Float (double-precision)"))
  (locals (WorldScale :type "Float (double-precision)" :default 5000.0))
  (bind _worldscale (`local.WorldScale`))
  (bind (_returnvalue_x _returnvalue_y) (`KismetMathLibrary.BreakVector` (- (`self.PrevActorLoc`) (`self.K2_GetActorLocation`))))
  (return (/ (`KismetMathLibrary.VSize2D` (`KismetMathLibrary.MakeVector2D` (/ _returnvalue_x _worldscale) (/ _returnvalue_y _worldscale))) `Delta Seconds`)) ; should return m/s
)

(fn `ChangeThrottle`
  (params (AxisValue :type "Float (double-precision)"))
  (locals (ThrottleScale :type "Float (double-precision)" :default 0.1))
  (bind _output_get (set `self.Throttle` (+ (`self.Throttle`) (* AxisValue (`local.ThrottleScale`)))))
  ;[1 1 1] Clamp Throttle to [-1,1] gets multiplied by force later
  (if (> _output_get 1.0)
    (set `self.Throttle` 1.0))
  (if (< _output_get -1.0)
    (set `self.Throttle` -1.0))
  (if false
    (`KismetSystemLibrary.PrintString` (`KismetStringLibrary.Conv_DoubleToString` (`self.Throttle`)) true true (struct :`G` 0.120274 :`B` 1.0 :`A` 1.0))))

(fn `UserConstructionScript`)