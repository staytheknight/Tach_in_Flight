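; BP_Wing2 is a simple player-controlled flight actor that moves along its static mesh's forward vector.
; Axis inputs adjust a clamped throttle that can go negative, accumulate pitch and yaw, and set a bank target from turn input.
; Tick advances a stored location by throttle times engine force without delta-time scaling or sweep, then sets mesh rotation directly, interpolating only roll for smooth banking.
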(event `self.ReceiveBeginPlay`
  (set `self.LocationDesired` (`SceneComponent.K2_GetComponentLocation` (`self.StaticMesh`))))

(event `self.ReceiveTick`
  (params (DeltaSeconds :type "Float (single-precision)"))
  (bind _returnvalue_roll (`KismetMathLibrary.BreakRotator` (`SceneComponent.K2_GetComponentRotation` (`self.StaticMesh`))))
  (bind _output_get (set `self.LocationDesired` (+ (`self.LocationDesired`) (* (* (`self.EngineForce`) (`self.Throttle`)) (`SceneComponent.GetForwardVector` (`self.StaticMesh`))))))
  (`self.K2_SetActorLocation` _output_get)
  (`SceneComponent.K2_SetWorldRotation` (`self.StaticMesh`) (`KismetMathLibrary.MakeRotator` (`KismetMathLibrary.FInterpTo` _returnvalue_roll (`self.Roll`) DeltaSeconds (`self.RInterpSpeed`)) (`self.Pitch`) (`self.Yaw`)) false false))

(event `InputAxis|InputAxis_Forward`
  (params (AxisValue :type "Float (single-precision)"))
  (`self.ChangeThrottle` AxisValue))

(event `InputAxis|InputAxis_Right_Arrows`
  (params (AxisValue :type "Float (single-precision)"))
  (`self.ChangeYaw` AxisValue)
  (set `self.Roll` (* AxisValue 90.0)))

(event `InputAxis|InputAxis_Forward_Arrows`
  (params (AxisValue :type "Float (single-precision)"))
  (`self.ChangePitch` AxisValue))

(fn `ChangePitch`
  (params (AxisValue :type "Float (double-precision)"))
  (bind _result (`/Engine/EditorBlueprintResources/StandardMacros.NegateFloat` AxisValue)
    (:`  `
      (set `self.Pitch` (+ (`self.Pitch`) _result)))))

(fn `ChangeThrottle`
  (params (AxisValue :type "Float (double-precision)"))
  (locals (ThrottleScale :type "Float (double-precision)" :default 0.1))
  (bind _output_get (set `self.Throttle` (+ (`self.Throttle`) (* AxisValue (`local.ThrottleScale`)))))
  ;[1 1 1] Clamp Throttle to [-1,1] gets multiplied by force later
  (if (> _output_get 1.0)
    (set `self.Throttle` 1.0))
  (if (< _output_get -1.0)
    (set `self.Throttle` -1.0))
  (if false
    (`KismetSystemLibrary.PrintString` (`KismetStringLibrary.Concat_StrStr` "Throttle: " (`KismetStringLibrary.Conv_DoubleToString` (`self.Throttle`))) true true (struct :`G` 0.120274 :`B` 1.0 :`A` 1.0))))

(fn `ChangeYaw`
  (params (AxisValue :type "Float (double-precision)"))
  (set `self.Yaw` (+ (`self.Yaw`) AxisValue)))

(fn `UserConstructionScript`)