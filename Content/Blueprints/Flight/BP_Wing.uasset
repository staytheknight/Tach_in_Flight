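; Flight physics prototype for a wing actor that applies thrust, lift and an impulse boost to its static mesh.
; Each tick adjusts throttle from axis input, then applies world-X thrust plus vertical gravity estimate and lift.
; Lift uses planar speed from position change in a simplified equation omitting area and coefficient.
; CalculateDrag is unused, and the throttle range check can overshoot [0,1] and stick.
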(event `self.ReceiveBeginPlay`
  (set `self.PrevActorLoc` (`self.K2_GetActorLocation`)))

(event `self.ReceiveTick`
  (params (DeltaSeconds :type "Float (single-precision)"))
  (`self.ChangeThrottle` (stale `InputAxis|InputAxis_Forward_Arrows` AxisValue))
  (`PrimitiveComponent.AddForce` (`self.StaticMesh`) (`self.CalculateForces` (`self.GravitationForceEstimate`) DeltaSeconds) "None" false)
  (set `self.PrevActorLoc` (`self.K2_GetActorLocation`)))

(event `InputAxis|InputAxis_Forward_Arrows`
  (params (AxisValue :type "Float (single-precision)")))

(event `InputAction|InputAction_Impulse`
  (params (Key :type "Key Structure"))
  (bind _impulse_strength (`self.Impulse Strength`))
  (bind (_returnvalue_x _returnvalue_y) (`KismetMathLibrary.BreakVector` (`SceneComponent.GetForwardVector` (`self.StaticMesh`))))
  (:`Pressed`
    (`PrimitiveComponent.AddImpulse` (`self.StaticMesh`) (`KismetMathLibrary.MakeVector` (* _returnvalue_x _impulse_strength) (* _returnvalue_y _impulse_strength)) "None" false)))

(fn `CalculateDrag`
  (params (`Obj Velocity` :type "Float (double-precision)") (DensityOfMedium :type "Float (double-precision)"))
  (returns (`Drag Force` :type "Float (double-precision)"))
  (return (* (`KismetMathLibrary.MultiplyMultiply_FloatFloat` `Obj Velocity` 2.0) (* DensityOfMedium 0.5))))

(fn `CalculateForces`
  (params (GraviationForce :type "Float (double-precision)") (DeltaSeconds :type "Float (double-precision)"))
  (returns (Vector :type "Vector Structure"))
  (locals (ThrottleForce :type "Float (double-precision)" :default 50000.0))
  (bind _velocity (`self.CalculatePlanarVelocity` DeltaSeconds))
  (bind _liftforce (`self.CalculateLiftForce` _velocity (`self.AIR_DENSITY`)))
  (bind _returnvalue (+ GraviationForce _liftforce))
  (if false
    (`KismetSystemLibrary.PrintString` (`KismetStringLibrary.Concat_StrStr` "Velocity: " (`KismetStringLibrary.Conv_DoubleToString` _velocity) " ,Lift Force: " (`KismetStringLibrary.Conv_DoubleToString` _liftforce) " ,Total Z Force: " (`KismetStringLibrary.Conv_DoubleToString` _returnvalue))))
  (return (`KismetMathLibrary.MakeVector` (* (`self.Throttle`) (`local.ThrottleForce`)) 0.0 _returnvalue)))

(fn `CalculateLiftForce`
  (params (ObjVelocity :type "Float (double-precision)") (DensityOfMedium :type "Float (double-precision)"))
  (returns (LiftForce :type "Float (double-precision)"))
  (return (* (`KismetMathLibrary.MultiplyMultiply_FloatFloat` ObjVelocity 2.0) (* DensityOfMedium 0.5))))

(fn `CalculatePlanarVelocity`
  (params (`Delta Seconds` :type "Float (double-precision)"))
  (returns (Velocity :type "Float (double-precision)"))
  (locals (WorldScale :type "Float (double-precision)" :default 50.0))
  (bind _worldscale (`local.WorldScale`))
  (bind (_returnvalue_x _returnvalue_y) (`KismetMathLibrary.BreakVector` (- (`self.PrevActorLoc`) (`self.K2_GetActorLocation`))))
  (return (/ (`KismetMathLibrary.VSize2D` (`KismetMathLibrary.MakeVector2D` (/ _returnvalue_x _worldscale) (/ _returnvalue_y _worldscale))) `Delta Seconds`)) ; should return m/s
)

(fn `ChangeThrottle`
  (params (AxisValue :type "Float (double-precision)"))
  (bind _throttle (`self.Throttle`))
  (if (and (<= _throttle 1.0) (>= _throttle 0.0))
    (set `self.Throttle` (+ _throttle AxisValue))))

(fn `UserConstructionScript`)